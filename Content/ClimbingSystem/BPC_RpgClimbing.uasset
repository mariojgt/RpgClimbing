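; Character component for wall climbing, with attach, surface movement, detach, ledge mantle and a basic teleport dash.
; Paired pelvis and head line traces validate the wall; attaching plays an air or floor montage, shrinks the capsule and uses Flying mode.
; MoveOnWall traces ahead to steer and align to the surface normal, mantling when the head trace misses or detaching at steep pitch.
; Tick, enabled while climbing, detaches when the wall is lost.
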(event `AttachToWall`
  (bind _characterref (`self.CharacterRef`))
  (bind _charactermovement (`Character.CharacterMovement` (`self.CharacterRef`)))
  ;[1 1 1] Wall attach start climbing
  (bind (_pelvishit _headhit _hithead) (`self.PelvisAndHeadTrace` (0.0 0.0 0.0)))
  ;;[1 1 1] Check if the character has hit the wall
  (if _hithead
    ;;[1 1 1] This fuction will check if the player is falling if yes play the fall grap montage
    (`self.PlayerGrabAllMontage`)
    (`MovementComponent.StopMovementImmediately` _charactermovement)
    (set `CharacterMovementComponent.bOrientRotationToMovement` false _charactermovement)
    (bind (_bblockinghit _binitialoverlap _time _distance _location _impactpoint _normal) (`GameplayStatics.BreakHitResult` _pelvishit))
    (bind _returnvalue (`KismetMathLibrary.MakeRotFromX` (* _normal -1.0)))
    ;;[1 1 1] Make the player face the wall
    (`Actor.K2_SetActorRotation` _characterref _returnvalue false)
    ;;[1 1 1] Player the grabAllMontage
    (`|PlayMontage` (`Character.Mesh` _characterref) (`self.Montage to Play`)
      (:`then`
        ;;[1 1 1] Move the player to the new location and disable the enable the is climbin and disable the movement
        (`KismetSystemLibrary.MoveComponentTo` (`Character.CapsuleComponent` _characterref) (+ _location (* _normal (`self.WallDistance`))) _returnvalue false false 0.0)
        (set `self.isClimbing` true)
        (`CharacterMovementComponent.DisableMovement` (`Character.CharacterMovement` (`self.CharacterRef`))))
      (:`OnCompleted`
        ;;[1 1 1] Once is complete we set the player movemnt mode and capsule
        (`CapsuleComponent.SetCapsuleHalfHeight` (`Character.CapsuleComponent` (`self.CharacterRef`)) 60.0 true)
        (`CharacterMovementComponent.SetMovementMode` (`Character.CharacterMovement` (`self.CharacterRef`)) "MOVE_Flying" 0)
        (`self.SetComponentTickEnabled` true)))
    (else
      (`KismetSystemLibrary.PrintString` "Surface not valid"))))

(event `self.ReceiveTick`
  (params (DeltaSeconds :type "Float (single-precision)"))
  (bind (_pelvishit _headhit _hithead) (`self.PelvisAndHeadTrace` (0.0 0.0 0.0)))
  ;[1 1 1] Check if the character has hit the wall
  (if (not _hithead)
    (`self.DeatchWall`)))

(event `DeatchWall`
  (bind _charactermovement (`Character.CharacterMovement` (`self.CharacterRef`)))
  ;[1 1 1] Wall detach
  (`CharacterMovementComponent.SetMovementMode` _charactermovement "MOVE_Falling" 0)
  (set `CharacterMovementComponent.bOrientRotationToMovement` true _charactermovement)
  (`Actor.K2_SetActorRotation` (`self.CharacterRef`) (`KismetMathLibrary.MakeRotator` 0.0) false)
  (`CapsuleComponent.SetCapsuleHalfHeight` (`Character.CapsuleComponent` (`self.CharacterRef`)) 96.0 true)
  (set `self.isClimbing` false)
  (`self.SetComponentTickEnabled` false))

(event `PlayerDash`
  (bind (_outhit _returnvalue) (`KismetSystemLibrary.LineTraceSingle` :`Start` (`Actor.K2_GetActorLocation` (`self.CharacterRef`)) :`End` (`self.NextDashLocation`) :`TraceChannel` "TraceTypeQuery1" :`DrawDebugType` "ForDuration"))
  (if (not _returnvalue)
    (`Actor.K2_SetActorLocationAndRotation` (`self.CharacterRef`) (`self.NextDashLocation`) (`self.PlayerLastRotation`) false false)
    (`self.AttachToWall`)))

(event `Move Up Ledge`
  (params (targetLocation :type "Vector Structure"))
  (bind (_playerlastrotation_roll _playerlastrotation_pitch _playerlastrotation_yaw) (`KismetMathLibrary.BreakRotator` (`self.PlayerLastRotation`)))
  (bind _characterref (`self.CharacterRef`))
  ;[1 1 1] This event will move the player up on the ledge
  (bind (_outhit _returnvalue) (`KismetSystemLibrary.CapsuleTraceSingle` targetLocation (+ targetLocation (* (`Actor.GetActorForwardVector` _characterref) (`self.MoveUpLedgeDistance`))) 30.0 (`CapsuleComponent.GetScaledCapsuleHalfHeight` (`Character.CapsuleComponent` _characterref)) "TraceTypeQuery1"))
  (if (not _returnvalue)
    (`|PlayMontage` (`Character.Mesh` (`self.CharacterRef`)) "/Game/ClimbingSystem/Animations/Animations/WallInteractions/MT_ClimbUp.MT_ClimbUp" 1.0 0.16
      (:`then`
        (`self.DeatchWall`)
        (`Actor.K2_SetActorRotation` (`self.CharacterRef`) (`KismetMathLibrary.MakeRotator` 0.0 0.0 _playerlastrotation_yaw) false)
        (`KismetSystemLibrary.MoveComponentTo` (`Character.CapsuleComponent` (`self.CharacterRef`)) (`.TraceEnd` (`GameplayStatics.BreakHitResult` _outhit)) (`KismetMathLibrary.MakeRotator` 0.0 0.0 _playerlastrotation_yaw) false false 0.4)
        (`CharacterMovementComponent.DisableMovement` (`Character.CharacterMovement` (`self.CharacterRef`))))
      (:`OnCompleted`
        (`CharacterMovementComponent.SetMovementMode` (`Character.CharacterMovement` (`self.CharacterRef`)) "MOVE_Walking" 0)))))

(fn `MoveOnWall`
  (params (AxisValue :type "Float (double-precision)") (VectorDiraction :type "Vector Structure"))
  (locals (`Vector Direction` :type "Vector Structure") (`move target` :type "Vector Structure") (ValueAxis :type "Float (double-precision)"))
  (bind _characterref (`self.CharacterRef`))
  (bind _returnvalue (`SceneComponent.GetSocketLocation` (`Character.Mesh` (`self.CharacterRef`)) (`self.MiddleBone`)))
  (bind _returnvalue_2 (+ _returnvalue (* (`local.Vector Direction`) (* (`local.ValueAxis`) 50.0))))
  (bind _output_get (set `local.ValueAxis` AxisValue))
  (set `self.LasPlayerAxis` _output_get)
  (set `local.Vector Direction` VectorDiraction)
  ;[1 1 1] Make sure the axis is not 0 if 0 do nothing
  (if (!= (`local.ValueAxis`) 0.0)
    (bind (_outhit _returnvalue_3) (`KismetSystemLibrary.CapsuleTraceSingle` _returnvalue _returnvalue_2 20.0 45.0 "TraceTypeQuery1"))
    (if _returnvalue_3
      (set `local.move target` (`.Location` (`GameplayStatics.BreakHitResult` _outhit)))
      (else
        (set `local.move target` _returnvalue_2)))
    (bind (_pelvishit _headhit _hithead _head) (`self.PelvisAndHeadTrace` (- (`local.move target`) (`SceneComponent.GetSocketLocation` (`Character.Mesh` (`self.CharacterRef`)) (`self.MiddleBone`)))))
    ;[1 1 1] Check if the head has hit something if yes we can stil move if no the player can climpb the ledge
    (if _hithead
      ;[1 1 1] For the future if we want to do a dash we can usig thi valriable
      (set `self.NextDashLocation` (+ (`local.move target`) (* (`local.Vector Direction`) (* (`local.ValueAxis`) 100.0))))
      (bind (_bblockinghit _binitialoverlap _time _distance _location _impactpoint _normal) (`GameplayStatics.BreakHitResult` _pelvishit))
      (`Pawn.AddMovementInput` _characterref (`KismetMathLibrary.GetDirectionUnitVector` (`Actor.K2_GetActorLocation` (`self.CharacterRef`)) (+ _location (* _normal (`self.WallDistance`)))) 1.0 false)
      (bind _returnvalue_4 (`KismetMathLibrary.RInterpTo` (`Actor.K2_GetActorRotation` (`self.CharacterRef`)) (`KismetMathLibrary.Conv_VectorToRotator` (* _normal -1.0)) (`GameplayStatics.GetWorldDeltaSeconds`) 2.0))
      (`Actor.K2_SetActorRotation` _characterref _returnvalue_4 false)
      ;[1 1 1] We going to use this in the climb
      (set `self.PlayerLastRotation` _returnvalue_4)
      ;[1 1 1] If the player pich rotaion is incalide detach from the wall and return to the original pitch
      (if (> (`KismetMathLibrary.Abs` (.pitch _returnvalue_4)) 70.0)
        (`self.DeatchWall`)
        (return))
      (else
        ;[1 1 1] Move up ledge
        (`self.Move Up Ledge` (+ _head (0.0 0.0 110.0)))))
    (else
      (return))))

(fn `PelvisAndHeadTrace`
  (params (offset :type "Vector Structure"))
  (returns (PelvisHit :type "HitResult Structure") (HeadHit :type "HitResult Structure") (hitHead :type Boolean) (Head :type "Vector Structure"))
  (bind _characterref (`self.CharacterRef`))
  (bind _returnvalue (* (`Actor.GetActorForwardVector` _characterref) 200.0))
  (bind _returnvalue_2 (+ (`Actor.K2_GetActorLocation` _characterref) offset))
  (bind _returnvalue_3 (+ (`SceneComponent.GetSocketLocation` (`Character.Mesh` _characterref) (`self.HeadBone`)) offset))
  (bind (_outhit _returnvalue_4) (`KismetSystemLibrary.LineTraceSingle` _returnvalue_2 (+ _returnvalue_2 _returnvalue) "TraceTypeQuery1"))
  (if _returnvalue_4
    (bind (_outhit_2 _returnvalue_5) (`KismetSystemLibrary.LineTraceSingle` _returnvalue_3 (+ _returnvalue_3 _returnvalue) "TraceTypeQuery1"))
    (return _outhit _outhit_2 _returnvalue_5 _returnvalue_3)
    (else
      (return (struct) (struct) false (0.0 0.0 0.0)))))

(fn `PlayerGrabAllMontage`
  (if (`NavMovementComponent.IsFalling` (`Character.CharacterMovement` (`self.CharacterRef`)))
    ;[1 1 1] If is falling
    (set `self.Montage to Play` "/Game/ClimbingSystem/Animations/Animations/WallInteractions/MT_AttachWallFromAir.MT_AttachWallFromAir")
    (else
      ;[1 1 1] Case in on the floor
      (set `self.Montage to Play` "/Game/ClimbingSystem/Animations/Animations/WallInteractions/MT_AttachWallFromFloor.MT_AttachWallFromFloor")))
  (return))