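; Actor component that handles a character's wall climbing transitions: attaching, detaching and mantling over a ledge.
; Forward line traces from actor location and head socket gate attaching, which switches to Flying, shrinks the capsule and moves it to face the wall.
; Detaching restores Falling, rotation to movement and capsule height.
; Ledge climbing runs a forward capsule trace from a supplied location and, if clear, detaches and moves the capsule forward.
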(event `AttachToWall`
  (bind _charactermovement (`Character.CharacterMovement` (`self.CharacterRef`)))
  (bind (_pelvishit _headhit _hithead) (`self.PelvisAndHeadTrace` (0.0 0.0 0.0)))
  (if _hithead
    (`CharacterMovementComponent.SetMovementMode` _charactermovement "MOVE_Flying" 0)
    (`MovementComponent.StopMovementImmediately` _charactermovement)
    (set `CharacterMovementComponent.bOrientRotationToMovement` false _charactermovement)
    (bind (_bblockinghit _binitialoverlap _time _distance _location _impactpoint _normal) (`GameplayStatics.BreakHitResult` _pelvishit))
    (`KismetSystemLibrary.MoveComponentTo` (`Character.CapsuleComponent` (`self.CharacterRef`)) (+ _location (* _normal (`self.WallDistance`))) (`KismetMathLibrary.MakeRotFromX` (* _normal -1.0)) false false 0.4)
    (`CapsuleComponent.SetCapsuleHalfHeight` (`Character.CapsuleComponent` (`self.CharacterRef`)) 60.0 true)))

(event `DeatchWall`
  (bind _charactermovement (`Character.CharacterMovement` (`self.CharacterRef`)))
  (`CharacterMovementComponent.SetMovementMode` _charactermovement "MOVE_Falling" 0)
  (set `CharacterMovementComponent.bOrientRotationToMovement` true _charactermovement)
  (`Actor.K2_SetActorRotation` (`self.CharacterRef`) (`KismetMathLibrary.MakeRotator` 0.0) false)
  (`CapsuleComponent.SetCapsuleHalfHeight` (`Character.CapsuleComponent` (`self.CharacterRef`)) 96.0 true))

(event `Move Up Ledge`
  (params (targetLocation :type "Vector Structure"))
  (bind _characterref (`self.CharacterRef`))
  (bind _characterref_2 (`self.CharacterRef`))
  (bind _returnvalue (+ targetLocation (* (`Actor.GetActorForwardVector` _characterref) 60.0)))
  (bind (_outhit _returnvalue_2) (`KismetSystemLibrary.CapsuleTraceSingle` :`Start` targetLocation :`End` _returnvalue :`Radius` 30.0 :`HalfHeight` (`CapsuleComponent.GetScaledCapsuleHalfHeight` (`Character.CapsuleComponent` _characterref)) :`TraceChannel` "TraceTypeQuery1" :`DrawDebugType` "ForDuration"))
  (if (not _returnvalue_2)
    (`self.DeatchWall`)
    (`KismetSystemLibrary.MoveComponentTo` (`Character.CapsuleComponent` _characterref_2) _returnvalue (`Actor.K2_GetActorRotation` _characterref_2))))

(fn `PelvisAndHeadTrace`
  (params (offset :type "Vector Structure"))
  (returns (PelvisHit :type "HitResult Structure") (HeadHit :type "HitResult Structure") (hitHead :type Boolean) (Head :type "Vector Structure"))
  (bind _characterref (`self.CharacterRef`))
  (bind _returnvalue (* (`Actor.GetActorForwardVector` _characterref) 200.0))
  (bind _returnvalue_2 (+ (`Actor.K2_GetActorLocation` _characterref) offset))
  (bind _returnvalue_3 (+ (`SceneComponent.GetSocketLocation` (`Character.Mesh` _characterref) "head") offset))
  (bind (_outhit _returnvalue_4) (`KismetSystemLibrary.LineTraceSingle` _returnvalue_2 (+ _returnvalue_2 _returnvalue) "TraceTypeQuery1"))
  (if _returnvalue_4
    (bind (_outhit_2 _returnvalue_5) (`KismetSystemLibrary.LineTraceSingle` _returnvalue_3 (+ _returnvalue_3 _returnvalue) "TraceTypeQuery1"))
    (return _outhit _outhit_2 _returnvalue_5 _returnvalue_3)))